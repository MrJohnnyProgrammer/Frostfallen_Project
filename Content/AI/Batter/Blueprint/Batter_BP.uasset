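; Batter enemy AI character that chases and attacks a visible player, feeding combat decisions to its Blackboard.
; While alive and seeing the player, Tick runs synchronous pathfinding into DirectionMovement, uses neck yaw and distance to flag strafe, random sword-down and axe attacks, and handles death.
; Custom events relay parry, kill and bat-hit reactions as Blackboard bools.
; The construction script makes clothing follow the body mesh via leader pose.
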(event `self.ReceiveBeginPlay`)

(event `self.ReceiveTick`
  (params (DeltaSeconds :type "Float (single-precision)"))
  (bind _neckrotyaw (`self.neckRotYaw`))
  (bind _returnvalue (`KismetMathLibrary.Vector_Distance` (`self.K2_GetActorLocation`) (`self.K2_GetActorLocation` (`GameplayStatics.GetPlayerCharacter` 0))))
  ;[1 1 1] event tick
  (if (and (`BlackboardComponent.GetValueAsBool` (`AIBlueprintHelperLibrary.GetBlackboard` null) "CanSeePlayer") (not (`self.bDead`)))
    (`|ExecutionSequence`
      (:`then_0`
        ;[1 1 1] path tracing
        (if (`BlackboardComponent.GetValueAsBool` (`AIBlueprintHelperLibrary.GetBlackboard` null) "CanSeePlayer")
          (`self.FindPath` (`self.endPoint`))
          (set `self.canSeePlayer` true)
          (else
            (set `self.canSeePlayer` false))))
      (:`then_1`
        ;[1 1 1] distance from player attack triggers
        (if (and (>= _neckrotyaw -30.0) (<= _neckrotyaw 30.0))
          (`BlackboardComponent.SetValueAsBool` (`AIBlueprintHelperLibrary.GetBlackboard` null) "FacingPlayer?" true)
          (if (not (`self.bAttacking`))
            (if (< _returnvalue 550.0)
              (`BlackboardComponent.SetValueAsBool` (`AIBlueprintHelperLibrary.GetBlackboard` null) "DoStrafe" true)
              (`|ExecutionSequence`
                (:`then_0`
                  (if (not (`self.bStrafing`))
                    (set `self.bStrafing` true)))
                (:`then_1`
                  (if (`KismetMathLibrary.NearlyEqual_FloatFloat` _returnvalue 400.0 5.0)
                    (if (< (`KismetMathLibrary.RandomInteger` 10) 4)
                      (`BlackboardComponent.SetValueAsBool` (`AIBlueprintHelperLibrary.GetBlackboard` null) "DoSwordDown" true)
                      (set `self.bLeftRight` (`KismetMathLibrary.RandomBool`))
                      (else
                        (if (< _returnvalue 200.0) :!label _label
                          (`BlackboardComponent.SetValueAsBool` (`AIBlueprintHelperLibrary.GetBlackboard` null) "DoAxeAttack" true)
                          (set `self.bLeftRight` (`KismetMathLibrary.RandomBool`))
                          (else
                            (`BlackboardComponent.SetValueAsBool` (`AIBlueprintHelperLibrary.GetBlackboard` null) "DoAxeAttack" false)))))
                    (else
                      (`BlackboardComponent.SetValueAsBool` (`AIBlueprintHelperLibrary.GetBlackboard` null) "DoSwordDown" false)
                      (goto _label)))))))
          (else
            (`BlackboardComponent.SetValueAsBool` (`AIBlueprintHelperLibrary.GetBlackboard` null) "FacingPlayer?" false))))
      (:`then_2`
        (if (<= (`self.health`) 0)
          (`BlackboardComponent.SetValueAsBool` (`AIBlueprintHelperLibrary.GetBlackboard` null) "IsDead" true)
          (`self.Death`)
          (`self.SetActorTickEnabled` false))))
    (else
      (set `self.enemyMovementStatus` "EMS_Idle"))))

(event `self.Parried`
  ;[1 1 1] bool events
  (`BlackboardComponent.SetValueAsBool` (`AIBlueprintHelperLibrary.GetBlackboard` null) "GotParried" true))

(event `self.Killed`
  ;[1 1 1] bool events
  (`BlackboardComponent.SetValueAsBool` (`AIBlueprintHelperLibrary.GetBlackboard` null) "IsDead" true))

(event `self.BodyParry`
  ;[1 1 1] bool events
  (`BlackboardComponent.SetValueAsBool` (`AIBlueprintHelperLibrary.GetBlackboard` null) "BodyParry" true))

(event `self.BatHitBP`
  ;[1 1 1] bool events
  (`BlackboardComponent.SetValueAsBool` (`AIBlueprintHelperLibrary.GetBlackboard` null) "batHit" true))

(fn `FindPath`
  (params (PathEnd :type "Vector Structure (by ref)"))
  (bind _returnvalue (`NavigationSystemV1.FindPathToLocationSynchronously` (`self.K2_GetActorLocation`) PathEnd (`AIBlueprintHelperLibrary.GetAIController` null) null))
  (`/Engine/EditorBlueprintResources/StandardMacros.IsValid` _returnvalue
    (:`Is Valid`
      (bind _pathpoints (`NavigationPath.PathPoints` _returnvalue))
      (if (> (`KismetArrayLibrary.Array_Length` _pathpoints) 0)
        (set `self.navPathIndex` 0)
        (`self.DirectionMovement` _pathpoints)))))

(fn `UserConstructionScript`
  (`SkinnedMeshComponent.SetLeaderPoseComponent` (`self.clothingSkeletalMesh`) (`self.Mesh`) false false))