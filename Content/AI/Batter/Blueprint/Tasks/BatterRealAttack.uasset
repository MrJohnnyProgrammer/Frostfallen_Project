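; Behavior tree task that makes the Batter AI perform its melee attack.
; It casts the controlled pawn to Batter_BP, then calls Attack when AxeEquipped is set or Kick otherwise.
; After a fixed delay it clears the BatAttack blackboard key and finishes successfully.
; An IsValid check on the equipped bat is left unconnected.
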(event `self.ReceiveExecuteAI`
  (params (OwnerController :type "AIController Object Reference") (ControlledPawn :type "Pawn Object Reference"))
  (bind _asbatter_bp (cast `/Game/AI/Batter/Blueprint/Batter_BP` ControlledPawn))
  (if (`Enemy.bAxeEquipped` _asbatter_bp)
    (`Marauder.Attack` _asbatter_bp)
    (else
      (`Marauder.Kick` _asbatter_bp)))
  (`KismetSystemLibrary.Delay` 1.8)
  (`BTFunctionLibrary.SetBlackboardValueAsBool` (`self.BatAttack`))
  (`self.FinishExecute` true))