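; Behavior tree task for the Batter AI that handles its reaction to being hit.
; It plays the pawn's bat hit animation, waits briefly, then swaps the mesh to the frozen material and flags it Frozen if it is not already.
; It then clears two blackboard bool keys and finishes successfully.
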(event `self.ReceiveExecuteAI`
  (params (OwnerController :type "AIController Object Reference") (ControlledPawn :type "Pawn Object Reference"))
  (bind _asbatter_bp (cast `/Game/AI/Batter/Blueprint/Batter_BP` ControlledPawn))
  (`Enemy.BatHitAnimation` _asbatter_bp)
  (`KismetSystemLibrary.Delay` 1.7)
  (if (not (`Enemy.bFrozen` _asbatter_bp))
    (`PrimitiveComponent.SetMaterial` (`Character.Mesh` _asbatter_bp) 0 (`Enemy.frozenMaterial` _asbatter_bp))
    (set `Enemy.bFrozen` true _asbatter_bp))
  (`BTFunctionLibrary.SetBlackboardValueAsBool` (`self.Key_0`))
  (`BTFunctionLibrary.SetBlackboardValueAsBool` (`self.NewVar_0`))
  (`self.FinishExecute` true))