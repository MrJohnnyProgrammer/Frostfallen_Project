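; Behavior tree task that handles the Marauder AI's reaction to being parried.
; It makes the controlled Marauder stumble and destroys its freeze aura component if one is valid.
; After a short delay it clears both the Parried and Kicked blackboard flags, then finishes successfully.
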(event `self.ReceiveExecuteAI`
  (params (OwnerController :type "AIController Object Reference") (ControlledPawn :type "Pawn Object Reference"))
  (bind _asmarauder_bp (cast `/Game/AI/Marauder/Blueprints/Marauder_BP` ControlledPawn))
  (`Marauder.Stumble` _asmarauder_bp)
  (bind _freezeaurasystem (`/Game/AI/Marauder/Blueprints/Marauder_BP.FreezeAuraSystem` _asmarauder_bp))
  (`/Engine/EditorBlueprintResources/StandardMacros.IsValid` _freezeaurasystem
    (:`Is Valid`
      (`ActorComponent.K2_DestroyComponent` _freezeaurasystem))
    (:`Is Not Valid`
      _))
  (`KismetSystemLibrary.Delay` 1.5)
  (`BTFunctionLibrary.SetBlackboardValueAsBool` (`self.Parried`))
  (`BTFunctionLibrary.SetBlackboardValueAsBool` (`self.Kicked`))
  (`self.FinishExecute` true))