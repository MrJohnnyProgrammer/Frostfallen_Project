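; Behavior tree task that makes the Marauder AI scream and then switch into its frozen state.
; After calling Scream on the controlled Marauder_BP, it waits briefly, swaps the mesh to the frozen material, triggers FreezeAura and sets the Frozen flag.
; It then clears the Scream blackboard key and finishes successfully; a failed pawn cast stops without finishing the task.
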(event `self.ReceiveExecuteAI`
  (params (OwnerController :type "AIController Object Reference") (ControlledPawn :type "Pawn Object Reference"))
  (bind _asmarauder_bp (cast `/Game/AI/Marauder/Blueprints/Marauder_BP` ControlledPawn))
  (`Marauder.Scream` _asmarauder_bp)
  (`KismetSystemLibrary.Delay` 2.0)
  (`PrimitiveComponent.SetMaterial` (`Character.Mesh` _asmarauder_bp) 0 (`Enemy.frozenMaterial` _asmarauder_bp))
  (`/Game/AI/Marauder/Blueprints/Marauder_BP.FreezeAura` _asmarauder_bp)
  (set `Enemy.bFrozen` true _asmarauder_bp)
  (`BTFunctionLibrary.SetBlackboardValueAsBool` (`self.Scream`))
  (`self.FinishExecute` true))