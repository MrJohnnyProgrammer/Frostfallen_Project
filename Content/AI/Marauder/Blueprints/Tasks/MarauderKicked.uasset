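; Behavior tree task that handles the Marauder enemy's reaction to being kicked.
; It makes the pawn stumble and drop its equipped axe, then sets the SpawnAxe blackboard key.
; After a short delay it clears the combat state keys for kicks, parries and attacks, then finishes successfully.
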(event `self.ReceiveExecuteAI`
  (params (OwnerController :type "AIController Object Reference") (ControlledPawn :type "Pawn Object Reference"))
  (bind _asmarauder_bp (cast `/Game/AI/Marauder/Blueprints/Marauder_BP` ControlledPawn))
  (`Marauder.Stumble` _asmarauder_bp)
  (`Axe.Drop` (`Enemy.equippedAxe` _asmarauder_bp))
  (`BTFunctionLibrary.SetBlackboardValueAsBool` (`self.SpawnAxe`) true)
  (`KismetSystemLibrary.Delay` 1.5)
  (`BTFunctionLibrary.SetBlackboardValueAsBool` (`self.Kicked`))
  (`BTFunctionLibrary.SetBlackboardValueAsBool` (`self.Parried`))
  (`BTFunctionLibrary.SetBlackboardValueAsBool` (`self.attack`))
  (`BTFunctionLibrary.SetBlackboardValueAsBool` (`self.attackdow`))
  (`BTFunctionLibrary.SetBlackboardValueAsBool` (`self.Kick`))
  (`self.FinishExecute` true))