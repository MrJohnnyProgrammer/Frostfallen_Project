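; Behavior tree task that drives the Marauder AI's movement when in fight range.
; On execute it sets the pawn's movement status to Sprint, calls its Strafe and RotateTowardsPlayer functions, then immediately finishes with success.
; Disconnected leftover nodes hold older logic that set EndPoint to the player's location or a diagonal left/right strafe point, and never run.
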(event `self.ReceiveExecuteAI`
  (params (OwnerController :type "AIController Object Reference") (ControlledPawn :type "Pawn Object Reference"))
  (bind _asmarauder_bp (cast `/Game/AI/Marauder/Blueprints/Marauder_BP` ControlledPawn))
  (set `Enemy.enemyMovementStatus` "EMS_Sprint" _asmarauder_bp)
  (`Enemy.Strafe` _asmarauder_bp)
  (`Enemy.RotateTowardsPlayer` _asmarauder_bp)
  (`self.FinishExecute` true))