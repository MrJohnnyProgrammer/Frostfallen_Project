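; AI controller for the Marauder enemy that runs Marauder_BT and feeds it perception of the player.
; Perception updates that cast to DefaultUnreal5Character_BP cache the character and write the CanSeePlayer and Player blackboard keys.
; The Player key stays set when sensing is lost, and GetPlayer exposes the cached reference.
; On BeginPlay, the brain component's tick is handed to TickOptToolkitMimic for tick optimization.
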(event `self.ReceiveBeginPlay`
  (`self.RunBehaviorTree` "/Game/AI/Marauder/Blueprints/Marauder_BT.Marauder_BT")
  (`TickOptToolkitMimicComponent.AddComponentTickControl` (`self.TickOptToolkitMimic`) (`self.BrainComponent`)))

(event `self.AIPerception.OnTargetPerceptionUpdated`
  (params (Actor :type "Actor Object Reference") (Stimulus :type "AIStimulus Structure"))
  (bind (_age _expirationage _strength _stimuluslocation _receiverlocation _tag _bsuccessfullysensed) (break `AIStimulus` Stimulus))
  (bind _asdefault_unreal_5character_bp (cast `/Game/ThirdPerson/Blueprints/DefaultUnreal5Character_BP` Actor))
  (set `self.Successfully Sensed` _bsuccessfullysensed)
  (bind _output_get (set `self.As Default Unreal 5Character BP` _asdefault_unreal_5character_bp))
  (`BlackboardComponent.SetValueAsBool` (`AIBlueprintHelperLibrary.GetBlackboard` null) "CanSeePlayer" _bsuccessfullysensed)
  (`BlackboardComponent.SetValueAsObject` (`AIBlueprintHelperLibrary.GetBlackboard` null) "Player" _output_get))

(fn `GetPlayer`
  (returns (`As Default Unreal 5Character BP` :type "/Game/ThirdPerson/Blueprints/DefaultUnreal5Character_BP Object Reference"))
  (return (`self.As Default Unreal 5Character BP`)))

(fn `UserConstructionScript`)