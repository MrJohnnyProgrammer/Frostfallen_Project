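; Axe-throwing enemy character that feeds its combat state to an AI Blackboard.
; While alive and seeing the player, Tick sets facing, strafe and kick flags from neck yaw and distance, and navmesh path points drive DirectionMovement.
; A head box catches axes thrown by others, attaching them and flagging a parry.
; Events relay axe possession, hits and parries to the Blackboard; zero health triggers death and stops Tick.
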(event `self.ReceiveBeginPlay`
  (`BlackboardComponent.SetValueAsBool` (`AIBlueprintHelperLibrary.GetBlackboard` null) "hasAxe?" false))

(event `self.ReceiveTick`
  (params (DeltaSeconds :type "Float (single-precision)"))
  (bind _neckrotyaw (`self.neckRotYaw`))
  (`|ExecutionSequence`
    (:`then_0`
      (if (and (`BlackboardComponent.GetValueAsBool` (`AIBlueprintHelperLibrary.GetBlackboard` null) "CanSeePlayer") (`|EnumInequality` (`self.enemyMovementStatus`) "EMS_Dead"))
        (`|ExecutionSequence`
          (:`then_0`
            (if (and (>= _neckrotyaw -20.0) (<= _neckrotyaw 20.0))
              ;[1 1 1] Detection
              (`BlackboardComponent.SetValueAsBool` (`AIBlueprintHelperLibrary.GetBlackboard` null) "FacingPlayer?" true)
              (if (<= (`KismetMathLibrary.Vector_Distance` (`self.K2_GetActorLocation`) (`self.K2_GetActorLocation` (`GameplayStatics.GetPlayerCharacter` 0))) 600.0)
                (`BlackboardComponent.SetValueAsBool` (`AIBlueprintHelperLibrary.GetBlackboard` null) "DoStrafe" true)
                (if (<= (`KismetMathLibrary.Vector_Distance` (`self.K2_GetActorLocation`) (`self.K2_GetActorLocation` (`GameplayStatics.GetPlayerCharacter` 0))) 150.0)
                  (`BlackboardComponent.SetValueAsBool` (`AIBlueprintHelperLibrary.GetBlackboard` null) "DoKick" true)
                  (else
                    (`BlackboardComponent.SetValueAsBool` (`AIBlueprintHelperLibrary.GetBlackboard` null) "DoKick" false)))
                (else
                  (`BlackboardComponent.SetValueAsBool` (`AIBlueprintHelperLibrary.GetBlackboard` null) "DoStrafe" false)))
              (else
                (`BlackboardComponent.SetValueAsBool` (`AIBlueprintHelperLibrary.GetBlackboard` null) "FacingPlayer?" false))))
          (:`then_1`
            ;[1 1 1] movement and rotation
            (set `self.canSeePlayer` true)
            (`self.Find Path` (`self.endPoint`))))
        (else
          (set `self.canSeePlayer` false))))
    (:`then_1`
      ;[1 1 1] Dying
      (if (<= (`self.health`) 0)
        (`BlackboardComponent.SetValueAsBool` (`AIBlueprintHelperLibrary.GetBlackboard` null) "IsDead" true)
        (`self.Death`)
        (`self.SetActorTickEnabled` false)))))

(event `self.Box1.OnComponentBeginOverlap`
  (params (OverlappedComponent :type "PrimitiveComponent Object Reference") (OtherActor :type "Actor Object Reference") (OtherComp :type "PrimitiveComponent Object Reference") (OtherBodyIndex :type Integer) (bFromSweep :type Boolean) (SweepResult :type "HitResult Structure (by ref)"))
  ;[1 1 1] Head oliision
  (if (not (`self.bAxeOnHead`))
    (bind _asaxe_bp (cast `/Game/PickUps/Axe_BP` OtherActor))
    (bind _output_get (set `self.headAxe` _asaxe_bp))
    (if (and (!= self (`Axe.axeHolder` _output_get)) (`Axe.bThrown` _output_get))
      (`BlackboardComponent.SetValueAsBool` (`AIBlueprintHelperLibrary.GetBlackboard` null) "axeOnHead?" true)
      (`BlackboardComponent.SetValueAsBool` (`AIBlueprintHelperLibrary.GetBlackboard` null) "GotParried" true)
      (`Axe.HeadAxeAttach` _output_get self "headSocket")
      (set `self.bAxeOnHead` true))))

(event `self.Killed`
  (`BlackboardComponent.SetValueAsBool` (`AIBlueprintHelperLibrary.GetBlackboard` null) "IsDead" true))

(event `self.axeOnHand`
  (params (on :type Boolean))
  (`BlackboardComponent.SetValueAsBool` (`AIBlueprintHelperLibrary.GetBlackboard` null) "hasAxe?" on))

(event `self.BodyParry`
  (`BlackboardComponent.SetValueAsBool` (`AIBlueprintHelperLibrary.GetBlackboard` null) "AxeThrowHit" true))

(event `self.BatHitBP`
  (`BlackboardComponent.SetValueAsBool` (`AIBlueprintHelperLibrary.GetBlackboard` null) "batHit" true))

(event `self.Parried`
  (`BlackboardComponent.SetValueAsBool` (`AIBlueprintHelperLibrary.GetBlackboard` null) "GotParried" true))

(fn `Find Path`
  (params (PathEnd :type "Vector Structure (by ref)"))
  (bind _returnvalue (`NavigationSystemV1.FindPathToLocationSynchronously` (`self.K2_GetActorLocation`) PathEnd (`AIBlueprintHelperLibrary.GetAIController` null) null))
  (`/Engine/EditorBlueprintResources/StandardMacros.IsValid` _returnvalue
    (:`Is Valid`
      (bind _pathpoints (`NavigationPath.PathPoints` _returnvalue))
      (if (> (`KismetArrayLibrary.Array_Length` _pathpoints) 0)
        (`self.DirectionMovement` _pathpoints)))))

(fn `UserConstructionScript`
  (`SkinnedMeshComponent.SetLeaderPoseComponent` (`self.clothingSkeletalMesh`) (`self.Mesh`) false false))