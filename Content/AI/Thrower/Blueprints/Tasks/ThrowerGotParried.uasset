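; Behavior tree task that handles the Thrower AI being parried.
; It calls Stumble on the Thrower and waits briefly, then freezes it by swapping in its frozen material and setting its Frozen flag, unless AxeOnHead is set.
; It then clears a boolean blackboard key and finishes successfully.
; A failed cast to Thrower_BP ends the event without finishing the task.
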(event `self.ReceiveExecuteAI`
  (params (OwnerController :type "AIController Object Reference") (ControlledPawn :type "Pawn Object Reference"))
  (bind _asthrower_bp (cast `/Game/AI/Thrower/Blueprints/Thrower_BP` ControlledPawn))
  (`Thrower.Stumble` _asthrower_bp)
  (`KismetSystemLibrary.Delay` 2.0)
  (if (not (`Thrower.bAxeOnHead` _asthrower_bp))
    (`PrimitiveComponent.SetMaterial` (`Character.Mesh` _asthrower_bp) 0 (`Enemy.frozenMaterial` _asthrower_bp))
    (set `Enemy.bFrozen` true _asthrower_bp))
  (`BTFunctionLibrary.SetBlackboardValueAsBool` (`self.NewVar_0`))
  (`self.FinishExecute` true)
  (`KismetSystemLibrary.PrintString` "Gotparried"))