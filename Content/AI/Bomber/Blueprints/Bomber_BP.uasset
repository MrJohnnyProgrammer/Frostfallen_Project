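; Bomber enemy AI character that reacts to seeing the player and to being parried through Blackboard flags.
; While alive and seeing the player, Tick runs a synchronous navmesh path query to EndPoint and passes the points to DirectionMovement.
; It also sets facing, walk and strafe flags from neck yaw and player distance.
; The construction script makes the clothing mesh follow the body's pose via Leader Pose.
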(event `self.ReceiveTick`
  (params (DeltaSeconds :type "Float (single-precision)"))
  (bind _neckrotyaw (`self.neckRotYaw`))
  (bind _returnvalue (`KismetMathLibrary.Vector_Distance` (`self.K2_GetActorLocation`) (`self.K2_GetActorLocation` (`GameplayStatics.GetPlayerCharacter` 0))))
  (if (and (`BlackboardComponent.GetValueAsBool` (`AIBlueprintHelperLibrary.GetBlackboard` null) "CanSeePlayer") (not (`self.bDead`)))
    (`|ExecutionSequence`
      (:`then_0`
        (`self.FindPath` (`self.endPoint`))
        (set `self.canSeePlayer` true))
      (:`then_1`
        (if (and (>= _neckrotyaw -20.0) (<= _neckrotyaw 20.0))
          (`BlackboardComponent.SetValueAsBool` (`AIBlueprintHelperLibrary.GetBlackboard` null) "FacingPlayer?" true)
          (else
            (`BlackboardComponent.SetValueAsBool` (`AIBlueprintHelperLibrary.GetBlackboard` null) "FacingPlayer?" false)))
        (if (>= _returnvalue 800.0)
          (`BlackboardComponent.SetValueAsBool` (`AIBlueprintHelperLibrary.GetBlackboard` null) "Walk" true)
          (else
            (`BlackboardComponent.SetValueAsBool` (`AIBlueprintHelperLibrary.GetBlackboard` null) "Walk" false)
            (if (<= _returnvalue 400.0)
              (`BlackboardComponent.SetValueAsBool` (`AIBlueprintHelperLibrary.GetBlackboard` null) "DoStrafe" true)
              (else
                (`BlackboardComponent.SetValueAsBool` (`AIBlueprintHelperLibrary.GetBlackboard` null) "DoStrafe" false)))))))
    (else
      (set `self.canSeePlayer` false))))

(event `self.Parried`
  (`BlackboardComponent.SetValueAsBool` (`AIBlueprintHelperLibrary.GetBlackboard` null) "GotParried" true))

(fn `FindPath`
  (params (PathEnd :type "Vector Structure (by ref)"))
  (bind _returnvalue (`NavigationSystemV1.FindPathToLocationSynchronously` (`self.K2_GetActorLocation`) PathEnd (`AIBlueprintHelperLibrary.GetAIController` null) null))
  (`/Engine/EditorBlueprintResources/StandardMacros.IsValid` _returnvalue
    (:`Is Valid`
      (bind _pathpoints (`NavigationPath.PathPoints` _returnvalue))
      (if (> (`KismetArrayLibrary.Array_Length` _pathpoints) 0)
        (set `self.navPathIndex` 0)
        (`self.DirectionMovement` _pathpoints)))))

(fn `UserConstructionScript`
  (`SkinnedMeshComponent.SetLeaderPoseComponent` (`self.clothingSkeletalMesh`) (`self.Mesh`) false false))