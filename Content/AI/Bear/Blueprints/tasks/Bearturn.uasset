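; Behavior tree task that makes the bear AI perform a turn.
; It calls Turn on Bear_BP with the blackboard's turn direction, temporarily allowing physics rotation during root motion.
; After a fixed delay rather than a completion callback, it clears the Turn key, sets Move, disables that rotation setting and finishes successfully.
; Unconnected nodes for clearing Move and rotating towards the player never run.
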(event `self.ReceiveExecuteAI`
  (params (OwnerController :type "AIController Object Reference") (ControlledPawn :type "Pawn Object Reference"))
  (bind _asbear_bp (cast `/Game/AI/Bear/Blueprints/Bear_BP` ControlledPawn))
  (bind _charactermovement (`Character.CharacterMovement` _asbear_bp))
  (set `CharacterMovementComponent.bAllowPhysicsRotationDuringAnimRootMotion` true _charactermovement)
  (`Bear.Turn` _asbear_bp (`BTFunctionLibrary.GetBlackboardValueAsBool` (`self.turnDirection`)))
  (`KismetSystemLibrary.Delay` 2.0)
  (`BTFunctionLibrary.SetBlackboardValueAsBool` (`self.turn`))
  (`BTFunctionLibrary.SetBlackboardValueAsBool` (`self.Move`) true)
  (set `CharacterMovementComponent.bAllowPhysicsRotationDuringAnimRootMotion` false _charactermovement)
  (`self.FinishExecute` true))