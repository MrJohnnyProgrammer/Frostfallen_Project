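; Behavior tree task that drives the bear's chase by pushing it forward while turning it toward the player.
; On execute it issues a simple move to a point a short distance along the pawn's facing, then calls RotateTowardsPlayer on Bear_BP.
; It finishes successfully at once without waiting for the move, then prints a debug string.
; A delay and a debug line trace remain as unconnected nodes.
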(event `self.ReceiveExecuteAI`
  (params (OwnerController :type "AIController Object Reference") (ControlledPawn :type "Pawn Object Reference"))
  (bind _asbear_bp (cast `/Game/AI/Bear/Blueprints/Bear_BP` ControlledPawn))
  (`AIBlueprintHelperLibrary.SimpleMoveToLocation` OwnerController (+ (`Actor.K2_GetActorLocation` ControlledPawn) (* (`KismetMathLibrary.GetForwardVector` (`Actor.K2_GetActorRotation` ControlledPawn)) 700.0)))
  (`Enemy.RotateTowardsPlayer` _asbear_bp)
  (`self.FinishExecute` true)
  (`KismetSystemLibrary.PrintString` "Hello"))