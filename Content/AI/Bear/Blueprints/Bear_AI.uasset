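; AI controller for the bear that runs its behavior tree and reports whether it senses the player.
; On BeginPlay it starts Bear_BT, then tries to cache its owner as Bear_BP.
; AI perception updates are filtered to DefaultUnreal5Character_BP, storing that character and writing the stimulus's sensed state to the CanSeePlayer blackboard key.
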(event `self.ReceiveBeginPlay`
  (`self.RunBehaviorTree` "/Game/AI/Bear/Blueprints/Bear_BT.Bear_BT")
  (bind _asbear_bp (cast `/Game/AI/Bear/Blueprints/Bear_BP` (`self.GetOwner`)))
  (set `self.As Bear BP` _asbear_bp))

(event `self.AIPerception.OnTargetPerceptionUpdated`
  (params (Actor :type "Actor Object Reference") (Stimulus :type "AIStimulus Structure"))
  (bind (_age _expirationage _strength _stimuluslocation _receiverlocation _tag _bsuccessfullysensed) (break `AIStimulus` Stimulus))
  (bind _asdefault_unreal_5character_bp (cast `/Game/ThirdPerson/Blueprints/DefaultUnreal5Character_BP` Actor))
  (set `self.Successfully Sensed` _bsuccessfullysensed)
  (set `self.As Default Unreal 5Character BP` _asdefault_unreal_5character_bp)
  (`BlackboardComponent.SetValueAsBool` (`AIBlueprintHelperLibrary.GetBlackboard` null) "CanSeePlayer" _bsuccessfullysensed))

(fn `UserConstructionScript`)