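; Bear enemy character with a second phase, whose Tick feeds attack and turn decisions to the AI Blackboard while it can see the player.
; Narrow distance bands flag charge, second-phase AOE, stomp or scratch, while Direction triggers turns and a rear AOE.
; FindPath passes a synchronous nav path to the player into DirectionMovement.
; Stomp, bite and paw overlaps damage the player; thrown axes attach to the head and flag a headshot.
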(event `self.ReceiveBeginPlay`
  (`BlackboardComponent.SetValueAsBool` (`AIBlueprintHelperLibrary.GetBlackboard` null) "Move" true))

(event `self.ReceiveTick`
  (params (DeltaSeconds :type "Float (single-precision)"))
  (bind _returnvalue (`AIBlueprintHelperLibrary.GetBlackboard` null))
  (bind _returnvalue_2 (`AIBlueprintHelperLibrary.GetBlackboard` null))
  (bind _direction (`self.Direction`))
  (bind _returnvalue_3 (`KismetMathLibrary.Vector_Distance` (`self.K2_GetActorLocation`) (`self.K2_GetActorLocation` (`GameplayStatics.GetPlayerCharacter` 0))))
  ;[1 1 1] Tick
  (`/Engine/EditorBlueprintResources/StandardMacros.IsValid` _returnvalue_2
    (:`Is Valid`
      (if (`BlackboardComponent.GetValueAsBool` _returnvalue_2 "CanSeePlayer")
        (`|ExecutionSequence`
          (:`then_0`
            ;[1 1 1] Distance detection
            (if (`KismetMathLibrary.NearlyEqual_FloatFloat` _returnvalue_3 1800.0 10.0)
              (`BlackboardComponent.SetValueAsBool` (`AIBlueprintHelperLibrary.GetBlackboard` null) "charge" true)
              (elif (`KismetMathLibrary.NearlyEqual_FloatFloat` _returnvalue_3 1200.0 10.0)
                (if (`self.2ndPhase`)
                  (`BlackboardComponent.SetValueAsBool` (`AIBlueprintHelperLibrary.GetBlackboard` null) "Aoe2" true))
                (elif (`KismetMathLibrary.NearlyEqual_FloatFloat` _returnvalue_3 500.0 50.0)
                  (`BlackboardComponent.SetValueAsBool` (`AIBlueprintHelperLibrary.GetBlackboard` null) "Stomp" true)
                  (elif (`KismetMathLibrary.NearlyEqual_FloatFloat` _returnvalue_3 400.0 25.0)
                    (`BlackboardComponent.SetValueAsBool` (`AIBlueprintHelperLibrary.GetBlackboard` null) "scratch" true))))))
          (:`then_1`
            ;[1 1 1] turn left right
            (if (> _direction 80.0)
              (`BlackboardComponent.SetValueAsBool` (`AIBlueprintHelperLibrary.GetBlackboard` null) "turn" true)
              (`BlackboardComponent.SetValueAsBool` (`AIBlueprintHelperLibrary.GetBlackboard` null) "left/right" false)
              (elif (< _direction -80.0)
                (`BlackboardComponent.SetValueAsBool` (`AIBlueprintHelperLibrary.GetBlackboard` null) "turn" true)
                (`BlackboardComponent.SetValueAsBool` (`AIBlueprintHelperLibrary.GetBlackboard` null) "left/right" true))))
          (:`then_2`
            ;[1 1 1] behind  AOE
            (if (and (> (`KismetMathLibrary.Abs` (`self.direction`)) 150.0) (`KismetMathLibrary.NearlyEqual_FloatFloat` (`KismetMathLibrary.Vector_Distance` (`self.K2_GetActorLocation`) (`self.K2_GetActorLocation` (`GameplayStatics.GetPlayerCharacter` 0))) 300.0 5.0))
              (`BlackboardComponent.SetValueAsBool` (`AIBlueprintHelperLibrary.GetBlackboard` null) "AOE" true)
              (`BlackboardComponent.SetValueAsBool` _returnvalue "scratch" false)
              (`BlackboardComponent.SetValueAsBool` _returnvalue "Stomp" false)))
          (:`then_3`
            ;[1 1 1] Getting Direction and Rotation
            (`self.FindPath`)
            (if (`CharacterMovementComponent.bAllowPhysicsRotationDuringAnimRootMotion` (`self.CharacterMovement`))
              _)))))))

(event `self.HeadCollision.OnComponentBeginOverlap`
  (params (OverlappedComponent :type "PrimitiveComponent Object Reference") (OtherActor :type "Actor Object Reference") (OtherComp :type "PrimitiveComponent Object Reference") (OtherBodyIndex :type Integer) (bFromSweep :type Boolean) (SweepResult :type "HitResult Structure (by ref)"))
  ;[1 1 1] head axe collision
  (bind _asaxe_bp (cast `/Game/PickUps/Axe_BP` OtherActor))
  (bind _output_get (set `self.headAxe` _asaxe_bp))
  (if (`Axe.bThrown` _output_get)
    (`BlackboardComponent.SetValueAsBool` (`AIBlueprintHelperLibrary.GetBlackboard` null) "headShot" true)
    (`Axe.HeadAxeAttach` (`self.headAxe`) self "headSocket")
    (set `self.bFrozen` false)))

(event `self.StompBox.OnComponentBeginOverlap`
  (params (OverlappedComponent :type "PrimitiveComponent Object Reference") (OtherActor :type "Actor Object Reference") (OtherComp :type "PrimitiveComponent Object Reference") (OtherBodyIndex :type Integer) (bFromSweep :type Boolean) (SweepResult :type "HitResult Structure (by ref)"))
  ;[1 1 1] attack collisions
  (bind _asdefault_unreal_5character_bp (cast `/Game/ThirdPerson/Blueprints/DefaultUnreal5Character_BP` OtherActor))
  (`GameplayStatics.ApplyDamage` _asdefault_unreal_5character_bp 8.0 (`self.GetController`) self "/Script/Engine.DamageType"))

(event `self.Body.OnComponentBeginOverlap`
  (params (OverlappedComponent :type "PrimitiveComponent Object Reference") (OtherActor :type "Actor Object Reference") (OtherComp :type "PrimitiveComponent Object Reference") (OtherBodyIndex :type Integer) (bFromSweep :type Boolean) (SweepResult :type "HitResult Structure (by ref)"))
  ;[1 1 1] attack collisions
)

(event `self.BiteCollision.OnComponentBeginOverlap`
  (params (OverlappedComponent :type "PrimitiveComponent Object Reference") (OtherActor :type "Actor Object Reference") (OtherComp :type "PrimitiveComponent Object Reference") (OtherBodyIndex :type Integer) (bFromSweep :type Boolean) (SweepResult :type "HitResult Structure (by ref)"))
  ;[1 1 1] attack collisions
  (bind _asdefault_unreal_5character_bp (cast `/Game/ThirdPerson/Blueprints/DefaultUnreal5Character_BP` OtherActor))
  (`GameplayStatics.ApplyDamage` _asdefault_unreal_5character_bp 8.0 (`self.GetController`) self "/Script/Engine.DamageType"))

(event `self.PawBox.OnComponentBeginOverlap`
  (params (OverlappedComponent :type "PrimitiveComponent Object Reference") (OtherActor :type "Actor Object Reference") (OtherComp :type "PrimitiveComponent Object Reference") (OtherBodyIndex :type Integer) (bFromSweep :type Boolean) (SweepResult :type "HitResult Structure (by ref)"))
  ;[1 1 1] attack collisions
  (bind _asdefault_unreal_5character_bp (cast `/Game/ThirdPerson/Blueprints/DefaultUnreal5Character_BP` OtherActor))
  (`GameplayStatics.ApplyDamage` _asdefault_unreal_5character_bp 8.0 (`self.GetController`) self "/Script/Engine.DamageType"))

(fn `FindPath`
  (bind _returnvalue (`NavigationSystemV1.FindPathToLocationSynchronously` (`self.K2_GetActorLocation`) (`self.K2_GetActorLocation` (`GameplayStatics.GetPlayerCharacter` 0)) (`AIBlueprintHelperLibrary.GetAIController` null) null))
  (`/Engine/EditorBlueprintResources/StandardMacros.IsValid` _returnvalue
    (:`Is Valid`
      (bind _pathpoints (`NavigationPath.PathPoints` _returnvalue))
      (if (> (`KismetArrayLibrary.Array_Length` _pathpoints) 0)
        (set `self.navPathIndex` 0)
        (`self.DirectionMovement` _pathpoints)))))

(fn `UserConstructionScript`)