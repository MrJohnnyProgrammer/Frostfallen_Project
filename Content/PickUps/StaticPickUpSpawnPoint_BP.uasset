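; StaticPickUpSpawnPoint_BP is a placeable spawn point that displays a chosen item: axe, bat, ice bomb, moon, hitable door or shearing door.
; The construction script checks the type flags in that priority order and makes the first match's component visible through a DoOnce.
; It never hides the other components, and the event graph is empty, so this Blueprint contains no spawning or pickup logic.
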(event `self.ReceiveTick`
  (params (DeltaSeconds :type "Float (single-precision)")))

(fn `UserConstructionScript`
  (if (`self.bAxe`)
    (`/Engine/EditorBlueprintResources/StandardMacros.DoOnce` false
      (:`Completed`
        (`SceneComponent.SetVisibility` (`self.Axe`) true false)))
    (elif (`self.bBat`)
      (`/Engine/EditorBlueprintResources/StandardMacros.DoOnce` false
        (:`Completed`
          (`SceneComponent.SetVisibility` (`self.Bat`) true false)))
      (elif (`self.bIceBombs`)
        (`/Engine/EditorBlueprintResources/StandardMacros.DoOnce` false
          (:`Completed`
            (`SceneComponent.SetVisibility` (`self.Bomb`) true false)))
        (elif (`self.bMoons`)
          (`/Engine/EditorBlueprintResources/StandardMacros.DoOnce` false
            (:`Completed`
              (`SceneComponent.SetVisibility` (`self.Moon`) true false)))
          (elif (`self.bHitableDoor`)
            (`/Engine/EditorBlueprintResources/StandardMacros.DoOnce` false
              (:`Completed`
                (`SceneComponent.SetVisibility` (`self.hDoor`) true false)))
            (elif (`self.bShearingDoor`)
              (`/Engine/EditorBlueprintResources/StandardMacros.DoOnce` false
                (:`Completed`
                  (`SceneComponent.SetVisibility` (`self.sDoor`) true false))))))))))